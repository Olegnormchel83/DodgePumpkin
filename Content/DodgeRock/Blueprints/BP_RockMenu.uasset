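; BP_RockMenu is a DodgeRock rock Blueprint, by its name meant for the menu, that supplies rotation helper functions.
; CreateRandomRotation returns small random positive roll and yaw values with zero pitch.
; TurnToPlayer points the actor's X axis at the first player pawn, if valid, using the normalized direction between their locations.
; BeginPlay and the construction script are empty, and neither function is called within this Blueprint.
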(event `self.ReceiveBeginPlay`)

(fn `CreateRandomRotation`
  (returns (RndRotation :type "Rotator Structure"))
  (bind _returnvalue (`KismetMathLibrary.RandomFloatInRange` 3.0 7.0))
  (return (`KismetMathLibrary.MakeRotator` _returnvalue 0.0 _returnvalue)))

(fn `UserConstructionScript`)