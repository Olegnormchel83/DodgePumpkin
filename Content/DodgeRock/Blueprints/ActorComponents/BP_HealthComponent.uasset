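; Health component for DodgeRock that tracks its owner's health, starting from a default value, and supports healing and timed invincibility.
; It binds to the owner's any-damage event, subtracts clamped damage, then broadcasts health changes and owner death at zero.
; AddHealth caps at default health without broadcasting.
; GiveInvincibility blocks damage until a timer ends it and destroys the DodgeRock character's ShieldFX component.
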(event `self.ReceiveBeginPlay`
  (add `Actor.OnTakeAnyDamage` (`self.GetOwner`) (delegate `OnTakeAnyDamage_Event`))
  (`self.SetHealth` (`self.DefaultHealth`)))

(event `OnTakeAnyDamage_Event`
  (params (DamagedActor :type "Actor Object Reference") (Damage :type "Float (single-precision)") (DamageType :type "DamageType Object Reference") (InstigatedBy :type "Controller Object Reference") (DamageCauser :type "Actor Object Reference"))
  (bind _health (`self.GetHealth`))
  (if (not (`self.IsInvincibility`))
    (`self.SetHealth` (`KismetMathLibrary.FClamp` (- _health Damage) 0.0 _health))
    (`self.HealthChanged`)
    (if (<= (`self.GetHealth`) 0.0)
      (`self.OnOwnerDied`))))

(event `GiveInvincibility`
  (set `self.IsInvincibility` true)
  (`KismetSystemLibrary.K2_SetTimerDelegate` (delegate `InvincibilityEnd`) (`self.InvincibilityTime`)))

(event `InvincibilityEnd`
  (set `self.IsInvincibility` false)
  (`self.K2_DestroyComponent` (`/Game/DodgeRock/Characters/BP_DodgeRockCharacter.ShieldFX` (cast `/Game/DodgeRock/Characters/BP_DodgeRockCharacter` (`self.GetOwner`) :!pure true))))

(fn `AddHealth`
  (params (Value :type "Float (double-precision)"))
  (`self.SetHealth` (`KismetMathLibrary.FClamp` (+ (`self.GetHealth`) Value) 0.0 (`self.DefaultHealth`))))

(fn `GetDefaultHealth`
  (returns (DefaultHealth :type "Float (double-precision)"))
  (return (`self.DefaultHealth`)))

(fn `GetHealth`
  (returns (Health :type "Float (double-precision)"))
  (return (`self.Health`)))

(fn `SetDefaultHealth`
  (params (NewDefaultHealth :type "Float (double-precision)"))
  (set `self.DefaultHealth` NewDefaultHealth))

(fn `SetHealth`
  (params (NewHealth :type "Float (double-precision)"))
  (set `self.Health` NewHealth))