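; BP_Heal is a moving heal pickup that heals actors implementing BPI_Pickupable on overlap.
; It turns toward the first player's pawn at BeginPlay, then moves forward each Tick with a swept offset.
; On hit, it re-aims along the hit actor's forward vector reflected off the surface normal, with pitch zeroed.
; On pickup, it sends the heal value through the interface, spawns particles and sound, then destroys itself.
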(event `self.ReceiveBeginPlay`
  (`|ExecutionSequence`
    (:`then_0`
      (`self.TurnToPlayer`))
    (:`then_1`
      (add `self.OnActorHit` (delegate `OnActorHit_Event`)))))

(event `OnActorHit_Event` :!signature `self.OnActorHit`
  (params (SelfActor :type "Actor Object Reference") (OtherActor :type "Actor Object Reference") (NormalImpulse :type "Vector Structure") (Hit :type "HitResult Structure (by ref)"))
  (bind (_returnvalue_roll _returnvalue_pitch _returnvalue_yaw) (`KismetMathLibrary.BreakRotator` (`KismetMathLibrary.MakeRotFromX` (`KismetMathLibrary.Vector_Normal2D` (`KismetMathLibrary.GetReflectionVector` (`self.GetActorForwardVector` OtherActor) (`.Normal` (`GameplayStatics.BreakHitResult` Hit)))))))
  (`self.K2_SetActorRotation` (`KismetMathLibrary.MakeRotator` _returnvalue_roll 0.0 _returnvalue_yaw)))

(event `self.ReceiveTick`
  (params (DeltaSeconds :type "Float (single-precision)"))
  (`self.K2_AddActorWorldOffset` (* (* DeltaSeconds (`self.Speed`)) (`self.GetActorForwardVector`)) true))

(event `self.Sphere.OnComponentBeginOverlap`
  (params (OverlappedComponent :type "PrimitiveComponent Object Reference") (OtherActor :type "Actor Object Reference") (OtherComp :type "PrimitiveComponent Object Reference") (OtherBodyIndex :type Integer) (bFromSweep :type Boolean) (SweepResult :type "HitResult Structure (by ref)"))
  (bind _returnvalue (`self.K2_GetActorLocation` OtherActor))
  (if (`KismetSystemLibrary.DoesImplementInterface` OtherActor "/Game/DodgeRock/Blueprints/Interfaces/BPI_Pickupable.BPI_Pickupable_C")
    (message `/Game/DodgeRock/Blueprints/Interfaces/BPI_Pickupable.PickupHeal` OtherActor (`self.HealValue`))
    (`GameplayStatics.SpawnEmitterAttached` "/Game/DodgeRock/VFX/P_Heal_Target.P_Heal_Target" OtherComp "None" _returnvalue (struct) (1.0 1.0 1.0) "KeepWorldPosition")
    (`GameplayStatics.SpawnSoundAtLocation` "/Game/DodgeRock/Sound/Cues/Effects/C_Heal.C_Heal" _returnvalue (struct) 1.0 1.0 0.0 null null)
    (`self.K2_DestroyActor`)))

(fn `UserConstructionScript`)