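; Spawner actor for the DodgeRock game that creates falling-hazard rocks and heal pickups at random points within a box volume.
; On BeginPlay it sets rock speed and damage from the game instance's difficulty and binds to the player's death.
; SpawnRockInVolume rolls against HealSpawnPercent to spawn a randomly rotated rock or a heal, both at actor height and rock speed.
; Player death destroys all rocks after a short delay.
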(event `self.ReceiveBeginPlay`
  (`|ExecutionSequence`
    (:`then_0`
      (bind _asbp_dodge_rock_game_instance (cast `/Game/DodgeRock/Core/GameInstances/BP_DodgeRockGameInstance` (`GameplayStatics.GetGameInstance`)))
      (`|ExecutionSequence`
        (:`then_0`
          (bind _gamedifficulty (`/Game/DodgeRock/Core/GameInstances/BP_DodgeRockGameInstance.GetGameDifficulty` _asbp_dodge_rock_game_instance))
          (set `self.RockDamage` (select `/Game/DodgeRock/Core/Enums/EGameDifficulty` _gamedifficulty :`NewEnumerator0` 10.0 :`NewEnumerator1` 20.0 :`NewEnumerator2` 34.0)))
        (:`then_1`
          (set `self.RockSpeed` (select `/Game/DodgeRock/Core/Enums/EGameDifficulty` _gamedifficulty :`NewEnumerator0` 750.0 :`NewEnumerator1` 1000.0 :`NewEnumerator2` 1500.0)))))
    (:`then_1`
      (bind _asbp_dodge_rock_character (cast `/Game/DodgeRock/Characters/BP_DodgeRockCharacter` (`GameplayStatics.GetPlayerPawn` 0)))
      (add `/Game/DodgeRock/Blueprints/ActorComponents/BP_HealthComponent.OnOwnerDied` (`/Game/DodgeRock/Characters/BP_DodgeRockCharacter.BP_HealthComponent` _asbp_dodge_rock_character) (delegate `OnPlayerDied_Event`)))))

(event `OnPlayerDied_Event`
  (`KismetSystemLibrary.Delay` 0.7)
  (bind _outactors (`GameplayStatics.GetAllActorsOfClass` "/Game/DodgeRock/Blueprints/BP_Rock.BP_Rock_C"))
  (for _array_element _outactors
    (`self.K2_DestroyActor` _array_element)))

(event `SpawnRockInVolume`
  (if (> (`KismetMathLibrary.RandomFloatInRange` 0.0 1.0) (`self.HealSpawnPercent`))
    (`self.SpawnRock`)
    (else
      (`self.SpawnHeal`))))

(fn `GetRandomSpawnRotation`
  (returns (SpawnRotation :type "Rotator Structure"))
  (bind _returnvalue (`KismetMathLibrary.RandomFloatInRange` 1.0 90.0))
  (return (`KismetMathLibrary.MakeRotator` _returnvalue _returnvalue _returnvalue)))

(fn `SpawnHeal`
  (bind (_returnvalue_x _returnvalue_y _returnvalue_z) (`KismetMathLibrary.BreakVector` (`self.K2_GetActorLocation`)))
  (bind _box (`self.Box`))
  (bind (_returnvalue_x_2 _returnvalue_y_2) (`KismetMathLibrary.BreakVector` (`KismetMathLibrary.RandomPointInBoundingBox` (`SceneComponent.K2_GetComponentLocation` _box) (`BoxComponent.BoxExtent` _box))))
  (`|SpawnActorFromClass` "/Game/DodgeRock/Blueprints/Pickups/BP_Heal.BP_Heal_C" (`KismetMathLibrary.MakeTransform` (`KismetMathLibrary.MakeVector` _returnvalue_x_2 _returnvalue_y_2 _returnvalue_z)) "AlwaysSpawn" "MultiplyWithRoot" null (`self.RockSpeed`) null))

(fn `SpawnRock`
  (bind (_returnvalue_x _returnvalue_y _returnvalue_z) (`KismetMathLibrary.BreakVector` (`self.K2_GetActorLocation`)))
  (bind _box (`self.Box`))
  (bind (_returnvalue_x_2 _returnvalue_y_2) (`KismetMathLibrary.BreakVector` (`KismetMathLibrary.RandomPointInBoundingBox` (`SceneComponent.K2_GetComponentLocation` _box) (`BoxComponent.BoxExtent` _box))))
  (`|SpawnActorFromClass` "/Game/DodgeRock/Blueprints/BP_Rock.BP_Rock_C" (`KismetMathLibrary.MakeTransform` (`KismetMathLibrary.MakeVector` _returnvalue_x_2 _returnvalue_y_2 _returnvalue_z) (`self.GetRandomSpawnRotation`)) "AdjustIfPossibleButAlwaysSpawn" "MultiplyWithRoot" null (`self.RockSpeed`) (`self.RockDamage`) null))

(fn `UserConstructionScript`)