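; BP_DodgeRockCharacter is the Dodge Rock character, handling level music and ragdoll death.
; BeginPlay starts the main level theme after a short delay and keeps a reference to it.
; When the health component reports death, it disables input, capsule collision and spring arm collision tests, ragdolls the mesh, sets a short lifespan and stops the music.
; While dead, Tick moves the actor to the simulated mesh's location.
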(event `self.ReceiveBeginPlay`
  (`KismetSystemLibrary.Delay` 0.8)
  (bind _returnvalue (`GameplayStatics.SpawnSound2D` "/Game/DodgeRock/Sound/Cues/C_MainLevelTheme.C_MainLevelTheme" 1.0 1.0 0.0 null false false))
  (set `self.LevelTheme` _returnvalue))

(event `self.BP_HealthComponent.OnOwnerDied`
  (bind _mesh (`self.Mesh`))
  (`|ExecutionSequence`
    (:`then_0`
      (set `self.IsDead` true)
      (`self.DisableInput` (`GameplayStatics.GetPlayerController` 0) null)
      (set `SpringArmComponent.bDoCollisionTest` false (`self.SpringArm`))
      (`PrimitiveComponent.SetCollisionEnabled` (`self.CapsuleComponent`) "NoCollision")
      (`PrimitiveComponent.SetCollisionEnabled` _mesh "QueryAndPhysics")
      (`PrimitiveComponent.SetSimulatePhysics` _mesh true)
      (`self.SetLifeSpan` 3.0))
    (:`then_1`
      (`AudioComponent.Stop` (`self.LevelTheme`)))))

(event `self.ReceiveTick`
  (params (DeltaSeconds :type "Float (single-precision)"))
  (if (`self.IsDead`)
    (`self.K2_SetActorLocation` (`SceneComponent.K2_GetComponentLocation` (`self.Mesh`)))))

(fn `UserConstructionScript`)