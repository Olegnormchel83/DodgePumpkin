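; Game state for the DodgeRock game that runs the round lifecycle of start, end and level-reload restart, and tracks rock count.
; On BeginPlay it caches the game mode and player state and sets points per tick from the game instance's difficulty.
; A looping one-second timer increments time played, adds score to the player state and passes elapsed time to the game mode.
; Ending the game clears the timer and submits the score as a high score.
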(event `self.ReceiveBeginPlay`
  (bind _asbp_dodge_rock_game_mode (cast `/Game/DodgeRock/Core/GameModes/BP_DodgeRockGameMode` (`GameplayStatics.GetGameMode`)))
  (set `self.DodgeRockGameMode` _asbp_dodge_rock_game_mode)
  (bind _asbp_dodge_rock_player_state (cast `/Game/DodgeRock/Core/PlayerStates/BP_DodgeRockPlayerState` (`GameplayStatics.GetPlayerState` 0)))
  (set `self.DodgeRockPlayerState` _asbp_dodge_rock_player_state)
  (bind _asbp_dodge_rock_game_instance (cast `/Game/DodgeRock/Core/GameInstances/BP_DodgeRockGameInstance` (`GameplayStatics.GetGameInstance`)))
  (set `self.PlayerPointsToAdd` (select `/Game/DodgeRock/Core/Enums/EGameDifficulty` (`/Game/DodgeRock/Core/GameInstances/BP_DodgeRockGameInstance.GetGameDifficulty` _asbp_dodge_rock_game_instance) :`NewEnumerator0` 1 :`NewEnumerator1` 3 :`NewEnumerator2` 7)))

(event `StartGame`
  (bind _returnvalue (`KismetSystemLibrary.K2_SetTimerDelegate` (`|CreateDelegate` :!event `CoreGameTimerEvent`) 1.0 true))
  (set `self.CoreGameTimer` _returnvalue)
  (set `self.bIsGameEnded` false))

(event `EndGame`
  (`KismetSystemLibrary.K2_ClearAndInvalidateTimerHandle` (`self.CoreGameTimer`))
  (set `self.bIsGameEnded` true)
  (bind _asbp_dodge_rock_game_instance (cast `/Game/DodgeRock/Core/GameInstances/BP_DodgeRockGameInstance` (`GameplayStatics.GetGameInstance`)))
  (bind _dodgerockplayerstate (`self.DodgeRockPlayerState`)
    (:`then`
      (`/Game/DodgeRock/Core/GameInstances/BP_DodgeRockGameInstance.SetHigherScore` _asbp_dodge_rock_game_instance (`/Game/DodgeRock/Core/PlayerStates/BP_DodgeRockPlayerState.GetPlayerScore` _dodgerockplayerstate)))
    (:`else`)))

(event `RestartGame`
  (bind _returnvalue (`GameplayStatics.GetCurrentLevelName` true))
  (`GameplayStatics.OpenLevel` (`KismetStringLibrary.Conv_StringToName` _returnvalue)))

(event `CoreGameTimerEvent`
  (`/Engine/EditorBlueprintResources/StandardMacros.IncrementInt` (`self.TimePlayed`)
    (:`  `
      (`|ExecutionSequence`
        (:`then_0`
          (bind _dodgerockplayerstate (`self.DodgeRockPlayerState`)
            (:`then`
              (`/Game/DodgeRock/Core/PlayerStates/BP_DodgeRockPlayerState.SetPlayerScore` _dodgerockplayerstate (+ (`/Game/DodgeRock/Core/PlayerStates/BP_DodgeRockPlayerState.GetPlayerScore` _dodgerockplayerstate) (`self.PlayerPointsToAdd`))))
            (:`else`)))
        (:`then_1`
          (bind _dodgerockgamemode (`self.DodgeRockGameMode`)
            (:`then`
              (`/Game/DodgeRock/Core/GameModes/BP_DodgeRockGameMode.Process` _dodgerockgamemode (`self.TimePlayed`)))
            (:`else`)))))))

(fn `GetRockCount`
  (returns (RockCount :type Integer))
  (return (`self.RockCount`)))

(fn `SetRockCount`
  (params (NewRockCount :type Integer))
  (set `self.RockCount` NewRockCount))

(fn `UserConstructionScript`)