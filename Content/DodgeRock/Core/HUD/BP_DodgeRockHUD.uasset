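; BP_DodgeRockHUD is the DodgeRock HUD, managing the player interface and death screen widgets.
; On BeginPlay it caches the player controller, shows WBP_PlayerInterface and binds to the owner-died event of the possessed character's health component.
; On death it removes the interface, shows WBP_DeathScreen, then switches to game-and-UI input focused on that screen with the mouse cursor visible.
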(event `self.ReceiveBeginPlay`
  (bind _asbp_dodge_rock_player_controller (cast `/Game/DodgeRock/Core/PlayerControllers/BP_DodgeRockPlayerController` (`GameplayStatics.GetPlayerController` 0)))
  (set `self.DodgeRockPlayerController` _asbp_dodge_rock_player_controller)
  (bind _returnvalue (`|CreateWidget` "/Game/DodgeRock/UI/Widgets/WBP_PlayerInterface.WBP_PlayerInterface_C" (`self.GetOwningPlayerController`)))
  (bind _output_get (set `self.PlayerInterfaceWidget` _returnvalue))
  (`UserWidget.AddToViewport` _output_get 0)
  (bind _asbp_dodge_rock_character (cast `/Game/DodgeRock/Characters/BP_DodgeRockCharacter` (`self.GetOwningPawn`)))
  (add `/Game/DodgeRock/Blueprints/ActorComponents/BP_HealthComponent.OnOwnerDied` (`/Game/DodgeRock/Characters/BP_DodgeRockCharacter.BP_HealthComponent` _asbp_dodge_rock_character) (delegate `OnOwnerDied_Event`)))

(event `OnOwnerDied_Event`
  (`|ExecutionSequence`
    (:`then_0`
      (bind _playerinterfacewidget (`self.PlayerInterfaceWidget`)
        (:`then`
          (`Widget.RemoveFromParent` _playerinterfacewidget))
        (:`else`)))
    (:`then_1`
      (bind _returnvalue (`|CreateWidget` "/Game/DodgeRock/UI/Widgets/WBP_DeathScreen.WBP_DeathScreen_C"))
      (bind _output_get (set `self.DeathScreenWidget` _returnvalue))
      (`UserWidget.AddToViewport` _output_get 0)
      (bind _dodgerockplayercontroller (`self.DodgeRockPlayerController`)
        (:`then`
          (`WidgetBlueprintLibrary.SetInputMode_GameAndUIEx` _dodgerockplayercontroller (`self.DeathScreenWidget`))
          (set `PlayerController.bShowMouseCursor` true _dodgerockplayercontroller))
        (:`else`)))))

(fn `UserConstructionScript`)