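; Game instance for DodgeRock that holds the game difficulty and the high score.
; Setter and getter functions expose both values to other code.
; The high score setter only stores a new value when it beats the current one.
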(fn `GetGameDifficulty`
  (returns (GameDifficulty :type "/Game/DodgeRock/Core/Enums/EGameDifficulty Enum"))
  (return (`self.GameDifficulty`)))

(fn `GetHigherScore`
  (returns (HigherScore :type Integer))
  (return (`self.HigherScore`)))

(fn `SetGameDifficulty`
  (params (Difficulty :type "/Game/DodgeRock/Core/Enums/EGameDifficulty Enum" :default "NewEnumerator0"))
  (set `self.GameDifficulty` Difficulty))

(fn `SetHigherScore`
  (params (NewHigherScore :type Integer))
  (if (> NewHigherScore (`self.GetHigherScore`))
    (set `self.HigherScore` NewHigherScore)))